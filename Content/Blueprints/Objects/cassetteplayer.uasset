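; VR cassette player prop with physical play/stop, next, previous and volume buttons, starting on a random song from SongList.
; Button overlaps forward to per-button interactive components, whose Pressed events drive one Audio component, with wraparound track selection and stepped, clamped volume.
; It records music playtime analytics on stop, and binds to MotionControllerPawn's quit event to report the last changed volume and, if playback was timed, playtime.
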(event OnComponentBeginOverlap(PlayBtn)
  (params (OverlappedComponent :type Primitive%20Component%20Object%20Reference) (OtherActor :type Actor%20Object%20Reference) (OtherComp :type Primitive%20Component%20Object%20Reference) (OtherBodyIndex :type Integer) (bFromSweep :type Boolean) (SweepResult :type Hit%20Result%20Structure%20%28by%20ref%29))
  (Default|ButtonBeginOverlap (Variables|Default|GetComp_InteractivePlay) OtherComp))

(event OnComponentEndOverlap(PlayBtn)
  (params (OverlappedComponent :type Primitive%20Component%20Object%20Reference) (OtherActor :type Actor%20Object%20Reference) (OtherComp :type Primitive%20Component%20Object%20Reference) (OtherBodyIndex :type Integer))
  (Default|ButtonEndOverlap (Variables|Default|GetComp_InteractivePlay) OtherComp))

(event OnComponentBeginOverlap(NextBtn)
  (params (OverlappedComponent :type Primitive%20Component%20Object%20Reference) (OtherActor :type Actor%20Object%20Reference) (OtherComp :type Primitive%20Component%20Object%20Reference) (OtherBodyIndex :type Integer) (bFromSweep :type Boolean) (SweepResult :type Hit%20Result%20Structure%20%28by%20ref%29))
  (Default|ButtonBeginOverlap (Variables|Default|GetComp_InteractiveNext) OtherComp))

(event OnComponentEndOverlap(NextBtn)
  (params (OverlappedComponent :type Primitive%20Component%20Object%20Reference) (OtherActor :type Actor%20Object%20Reference) (OtherComp :type Primitive%20Component%20Object%20Reference) (OtherBodyIndex :type Integer))
  (Default|ButtonEndOverlap (Variables|Default|GetComp_InteractiveNext) OtherComp))

(event OnComponentBeginOverlap(PrevBtn)
  (params (OverlappedComponent :type Primitive%20Component%20Object%20Reference) (OtherActor :type Actor%20Object%20Reference) (OtherComp :type Primitive%20Component%20Object%20Reference) (OtherBodyIndex :type Integer) (bFromSweep :type Boolean) (SweepResult :type Hit%20Result%20Structure%20%28by%20ref%29))
  (Default|ButtonBeginOverlap (Variables|Default|GetComp_InteractivePrev) OtherComp))

(event OnComponentEndOverlap(PrevBtn)
  (params (OverlappedComponent :type Primitive%20Component%20Object%20Reference) (OtherActor :type Actor%20Object%20Reference) (OtherComp :type Primitive%20Component%20Object%20Reference) (OtherBodyIndex :type Integer))
  (Default|ButtonEndOverlap (Variables|Default|GetComp_InteractivePrev) OtherComp))

(event OnComponentBeginOverlap(VolUpBtn)
  (params (OverlappedComponent :type Primitive%20Component%20Object%20Reference) (OtherActor :type Actor%20Object%20Reference) (OtherComp :type Primitive%20Component%20Object%20Reference) (OtherBodyIndex :type Integer) (bFromSweep :type Boolean) (SweepResult :type Hit%20Result%20Structure%20%28by%20ref%29))
  (Default|ButtonBeginOverlap (Variables|Default|GetComp_InteractiveVolUp) OtherComp))

(event OnComponentEndOverlap(VolUpBtn)
  (params (OverlappedComponent :type Primitive%20Component%20Object%20Reference) (OtherActor :type Actor%20Object%20Reference) (OtherComp :type Primitive%20Component%20Object%20Reference) (OtherBodyIndex :type Integer))
  (Default|ButtonEndOverlap (Variables|Default|GetComp_InteractiveVolUp) OtherComp))

(event OnComponentBeginOverlap(VolDownBtn)
  (params (OverlappedComponent :type Primitive%20Component%20Object%20Reference) (OtherActor :type Actor%20Object%20Reference) (OtherComp :type Primitive%20Component%20Object%20Reference) (OtherBodyIndex :type Integer) (bFromSweep :type Boolean) (SweepResult :type Hit%20Result%20Structure%20%28by%20ref%29))
  (Default|ButtonBeginOverlap (Variables|Default|GetComp_InteractiveVolDown) OtherComp))

(event OnComponentEndOverlap(VolDownBtn)
  (params (OverlappedComponent :type Primitive%20Component%20Object%20Reference) (OtherActor :type Actor%20Object%20Reference) (OtherComp :type Primitive%20Component%20Object%20Reference) (OtherBodyIndex :type Integer))
  (Default|ButtonEndOverlap (Variables|Default|GetComp_InteractiveVolDown) OtherComp))

(event Custom|VolDownEvent
  (bind _audio (Variables|Default|GetAudio))
  (bind _volumemultiplier (Variables|/Script/Engine.AudioComponent|GetVolumeMultiplier _audio))
  (bind _returnvalue (- _volumemultiplier 0.1))
  ;[1 1 1] VolDown
  (if (not (< _returnvalue 0.1))
    (Audio|Components|Audio|SetVolumeMultiplier _audio _returnvalue :!class /Script/Engine.AudioComponent)
    (Variables|Default|SetCurrentVolume (Variables|/Script/Engine.AudioComponent|GetVolumeMultiplier (Variables|Default|GetAudio)))))

(event Custom|VolUpEvent
  (bind _audio (Variables|Default|GetAudio))
  (bind _volumemultiplier (Variables|/Script/Engine.AudioComponent|GetVolumeMultiplier _audio))
  (bind _returnvalue (+ _volumemultiplier 0.1))
  ;[1 1 1] VolUp
  (if (not (> _returnvalue 1.0))
    (Audio|Components|Audio|SetVolumeMultiplier _audio _returnvalue :!class /Script/Engine.AudioComponent)
    (Variables|Default|SetCurrentVolume (Variables|/Script/Engine.AudioComponent|GetVolumeMultiplier (Variables|Default|GetAudio)))))

(event Custom|PlayEvent
  (bind _audio (Variables|Default|GetAudio))
  ;[1 1 1] playBtn
  (if (Audio|Components|Audio|IsPlaying _audio)
    (Audio|Components|Audio|Stop _audio)
    (CallFunction|AnalyitcsRecordMusicSession)
    (else
      (Audio|Components|Audio|Play _audio 0.0)
      (Variables|Default|SetMusicStartTimestamp (Actor|GetGameTimeSinceCreation)))))

(event Custom|NextEvent
  (bind _songlist (Variables|Default|GetSongList))
  ;[1 1 1] NextBtn
  (if (Utilities|Array|IsValidIndex _songlist (+ (Variables|Default|GetcurrentSongIndex) 1))
    (Variables|Default|SetcurrentSongIndex (+ (Variables|Default|GetcurrentSongIndex) 1))
    (else
      (Variables|Default|SetcurrentSongIndex 0)))
  (Audio|Components|Audio|SetSound (Variables|Default|GetAudio) (Utilities|Array|Get(acopy) _songlist (Variables|Default|GetcurrentSongIndex))))

(event Custom|PrevEvent
  (bind _songlist (Variables|Default|GetSongList))
  ;[1 1 1] PrevBtn
  (if (Utilities|Array|IsValidIndex _songlist (- (Variables|Default|GetcurrentSongIndex) 1))
    (Variables|Default|SetcurrentSongIndex (- (Variables|Default|GetcurrentSongIndex) 1))
    (else
      (Variables|Default|SetcurrentSongIndex (- (Utilities|Array|Length _songlist) 1))))
  (Audio|Components|Audio|SetSound (Variables|Default|GetAudio) (Utilities|Array|Get(acopy) _songlist (Variables|Default|GetcurrentSongIndex))))

(event Custom|Analyitcs_RecordMusicSession
  (bind _returnvalue (Actor|GetGameTimeSinceCreation))
  (bind _musicstarttimestamp (Variables|Default|GetMusicStartTimestamp))
  (bind _returnvalue_2 (- _returnvalue _musicstarttimestamp))
  (bind _returnvalue_3 (Utilities|String|ToString(Float) _returnvalue_2))
  ;[1 1 1] Record Music Session
  (Class|AnalyticsBlueprintLibrary|RecordEventwithAttribute "PlayerAction:Tapeplayer:MusicStopped" "Playtime" _returnvalue_3)
  (Development|PrintString (Utilities|String|Append "PlayerAction:Tapeplayer:MusicStopped - Playtime: " _returnvalue_3)))

(event Custom|SendLastVolumeValue
  (bind _currentvolume (Variables|Default|GetCurrentVolume))
  (if (!= _currentvolume -1.0)
    (Class|AnalyticsBlueprintLibrary|RecordEvent (Utilities|String|Append "PlayerAction:LastSetMusicVol:" (Utilities|String|ToString(Float) _currentvolume)))
    (if (!= (Variables|Default|GetMusicStartTimestamp) 0.0)
      (CallFunction|AnalyitcsRecordMusicSession))))

(event EventBeginPlay
  (bind _songlist (Variables|Default|GetSongList))
  (bind _comp_interactivenext (Variables|Default|GetComp_InteractiveNext))
  (bind _comp_interactiveprev (Variables|Default|GetComp_InteractivePrev))
  (bind _comp_interactiveplay (Variables|Default|GetComp_InteractivePlay))
  (bind _comp_interactivevolup (Variables|Default|GetComp_InteractiveVolUp))
  (bind _comp_interactivevoldown (Variables|Default|GetComp_InteractiveVolDown))
  (bind _audio (Variables|Default|GetAudio))
  (|CallParentFunction)
  (Utilities|FlowControl|Sequence
    (:then_0
      ;[1 1 1] Start off random song
      (bind _output_get (Variables|Default|SetcurrentSongIndex (Math|Random|RandomIntegerinRange 0 (- (Utilities|Array|Length _songlist) 1))))
      (Audio|Components|Audio|SetSound _audio (Utilities|Array|Get(acopy) _songlist _output_get))
      (if (Variables|Default|GetShouldPlayOnStart)
        (Audio|Components|Audio|Play _audio 0.0)))
    (:then_1
      (Utilities|FlowControl|Sequence
        (:then_0
          ;[1 1 1] playBtn
          (Variables|/Game/Blueprints/InteractiveObjects/Comp_InteractiveButton.Comp_InteractiveButton_C|SetButton _comp_interactiveplay (Variables|Default|GetPlayBtn))
          (Variables|/Game/Blueprints/InteractiveObjects/Comp_InteractiveButton.Comp_InteractiveButton_C|SetButtonRoot _comp_interactiveplay (Variables|Default|GetPlayRoot))
          (Variables|/Game/Blueprints/InteractiveObjects/Comp_InteractiveButton.Comp_InteractiveButton_C|SetButtonSound _comp_interactiveplay (Variables|Default|GetBtnClick))
          (EventDispatchers|BindEventtoPressed _comp_interactiveplay (delegate Custom|PlayEvent)))
        (:then_1
          ;[1 1 1] NextBtn
          (Variables|/Game/Blueprints/InteractiveObjects/Comp_InteractiveButton.Comp_InteractiveButton_C|SetButton _comp_interactivenext (Variables|Default|GetNextBtn))
          (Variables|/Game/Blueprints/InteractiveObjects/Comp_InteractiveButton.Comp_InteractiveButton_C|SetButtonRoot _comp_interactivenext (Variables|Default|GetNextRoot))
          (Variables|/Game/Blueprints/InteractiveObjects/Comp_InteractiveButton.Comp_InteractiveButton_C|SetButtonSound _comp_interactivenext (Variables|Default|GetBtnClick))
          (EventDispatchers|BindEventtoPressed _comp_interactivenext (delegate Custom|NextEvent)))
        (:then_2
          ;[1 1 1] PrevBtn
          (Variables|/Game/Blueprints/InteractiveObjects/Comp_InteractiveButton.Comp_InteractiveButton_C|SetButton _comp_interactiveprev (Variables|Default|GetPrevBtn))
          (Variables|/Game/Blueprints/InteractiveObjects/Comp_InteractiveButton.Comp_InteractiveButton_C|SetButtonRoot _comp_interactiveprev (Variables|Default|GetPrevRoot))
          (Variables|/Game/Blueprints/InteractiveObjects/Comp_InteractiveButton.Comp_InteractiveButton_C|SetButtonSound _comp_interactiveprev (Variables|Default|GetBtnClick))
          (EventDispatchers|BindEventtoPressed _comp_interactiveprev (delegate Custom|PrevEvent)))
        (:then_3
          ;[1 1 1] VolUp
          (Variables|/Game/Blueprints/InteractiveObjects/Comp_InteractiveButton.Comp_InteractiveButton_C|SetButton _comp_interactivevolup (Variables|Default|GetVolUpBtn))
          (Variables|/Game/Blueprints/InteractiveObjects/Comp_InteractiveButton.Comp_InteractiveButton_C|SetButtonRoot _comp_interactivevolup (Variables|Default|GetVolUpRoot))
          (Variables|/Game/Blueprints/InteractiveObjects/Comp_InteractiveButton.Comp_InteractiveButton_C|SetButtonSound _comp_interactivevolup (Variables|Default|GetBtnClick))
          (EventDispatchers|BindEventtoPressed _comp_interactivevolup (delegate Custom|VolUpEvent)))
        (:then_4
          ;[1 1 1] VolDown
          (Variables|/Game/Blueprints/InteractiveObjects/Comp_InteractiveButton.Comp_InteractiveButton_C|SetButton _comp_interactivevoldown (Variables|Default|GetVolDownBtn))
          (Variables|/Game/Blueprints/InteractiveObjects/Comp_InteractiveButton.Comp_InteractiveButton_C|SetButtonRoot _comp_interactivevoldown (Variables|Default|GetVolDownRoot))
          (Variables|/Game/Blueprints/InteractiveObjects/Comp_InteractiveButton.Comp_InteractiveButton_C|SetButtonSound _comp_interactivevoldown (Variables|Default|GetBtnClick))
          (EventDispatchers|BindEventtoPressed _comp_interactivevoldown (delegate Custom|VolDownEvent)))))
    (:then_2
      (bind _outactors (Actor|GetAllActorsOfClass "/Game/Blueprints/MotionControllerPawn.MotionControllerPawn_C"))
      (Utilities|IsValid (Utilities|Array|Get(acopy) _outactors)
        (:Is%20Valid
          (EventDispatchers|BindEventtoOnQuitGame (Utilities|Array|Get(acopy) _outactors) (delegate Custom|SendLastVolumeValue)))))))

(fn ConstructionScript
  (|CallParentFunction))