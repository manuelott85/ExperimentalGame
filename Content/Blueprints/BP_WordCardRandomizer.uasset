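; BP_WordCardRandomizer is an actor that hands out random words to the BP_WordCard actors in the level.
; On BeginPlay it loops over every BP_WordCard, picks a random entry from WordList and sets that card's TextRender text.
; Each used word is removed from the list, so no entry repeats, and cards left over once the list empties keep their existing text.
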(event EventBeginPlay
  (bind _wordlist (Variables|Default|GetWordList))
  (bind _outactors (Actor|GetAllActorsOfClass "/Game/Blueprints/BP_WordCard.BP_WordCard_C"))
  (for _array_element _outactors
    ;[1 1 1] Only proceed if there are enough words
    (if (> (Utilities|Array|Length (Variables|Default|GetWordList)) 0)
      (Variables|Default|SetchosenIndex (Math|Random|RandomIntegerinRange 0 (- (Utilities|Array|Length _wordlist) 1)))
      (Rendering|Components|TextRender|SetText (Variables|/Game/Blueprints/BP_WordCard.BP_WordCard_C|GetTextRender _array_element) (Utilities|Array|Get(acopy) _wordlist (Variables|Default|GetchosenIndex)))
      (Utilities|Array|RemoveIndex _wordlist (Variables|Default|GetchosenIndex)))))

(event Collision|EventActorBeginOverlap
  (params (OtherActor :type Actor%20Object%20Reference)))

(event EventTick
  (params (DeltaSeconds :type Float%20%28single-precision%29)))

(fn ConstructionScript)