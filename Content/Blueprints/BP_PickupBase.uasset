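; BP_PickupBase is a base physics pickup that attaches to a supplied component and detaches on drop, zeroing momentum below given thresholds.
; It starts with gravity on and hover suspended; pickup disables gravity and restores hover, which Tick drives through a timeline-based mesh offset.
; If respawn is enabled, the first pickup spawns a replacement at the saved spawn transform.
; Actor and mesh hit events play separate impact sounds without retriggering.
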(event OnComponentBeginOverlap(StaticMesh)
  (params (OverlappedComponent :type Primitive%20Component%20Object%20Reference) (OtherActor :type Actor%20Object%20Reference) (OtherComp :type Primitive%20Component%20Object%20Reference) (OtherBodyIndex :type Integer) (bFromSweep :type Boolean) (SweepResult :type Hit%20Result%20Structure%20%28by%20ref%29)))

(event OnComponentHit(StaticMesh)
  (params (HitComponent :type Primitive%20Component%20Object%20Reference) (OtherActor :type Actor%20Object%20Reference) (OtherComp :type Primitive%20Component%20Object%20Reference) (NormalImpulse :type Vector :default "0, 0, 0") (Hit :type Hit%20Result%20Structure%20%28by%20ref%29))
  (bind _objectcollidewhileinhand (Variables|Default|GetObjectCollideWhileInHand))
  (if (not (Audio|Components|Audio|IsPlaying _objectcollidewhileinhand))
    (Audio|Components|Audio|Play _objectcollidewhileinhand 0.0)))

(event Custom|OnImpactSound
  (params (SelfActor :type Actor%20Object%20Reference) (OtherActor :type Actor%20Object%20Reference) (NormalImpulse :type Vector) (Hit :type Hit%20Result%20Structure%20%28by%20ref%29))
  (bind _objectimpact (Variables|Default|GetObjectImpact))
  (Development|PrintString "Hello")
  (if (not (Audio|Components|Audio|IsPlaying _objectimpact))
    (Audio|Components|Audio|Play _objectimpact 0.0)))

(event EventBeginPlay
  (bind _hoveringamount (Variables|Hovering|GetHoveringAmount))
  (bind _staticmesh (Variables|Default|GetStaticMesh))
  ;[1 1 1] Event Play
  (Utilities|FlowControl|Sequence
    (:then_0
      ;[1 1 1] Save SpawnPosition
      (Variables|Default|SetSpawnTransform (Transformation|GetActorTransform))
      ;[1 1 1] Activate Physics at game start
      (Utilities|IsValid _staticmesh
        (:Is%20Valid
          (Physics|SetSimulatePhysics _staticmesh true)
          (Physics|SetEnableGravity _staticmesh false)
          (Physics|SetPhysicsLinearVelocity _staticmesh "0, 0, 0" false "None")
          (Class|PrimitiveComponent|SetPhysicsAngularVelocityinDegrees _staticmesh "0, 0, 0" false "None"))))
    (:then_1
      ;[1 1 1] Hover
      (bind _floatalpha (Timeline|FloatingTimeline SetNewTime)
        (:Update
          (Transformation|AddWorldOffset (Variables|Default|GetStaticMesh) (Math|Vector|MakeVector (* _floatalpha (.x _hoveringamount)) (* _floatalpha (.y _hoveringamount)) (* _floatalpha (.z _hoveringamount))) true false))))
    (:then_2
      ;[1 1 1] Activate gravity and deactivate hover by default
      (Physics|SetEnableGravity (Variables|Default|GetStaticMesh) true)
      (Variables|Hovering|SetShouldHoverStorage (Variables|Hovering|GetShouldHover))
      (Variables|Hovering|SetShouldHover false))
    (:then_3
      (EventDispatchers|AssignOnActorHit (delegate Custom|OnImpactSound)))))

(event EventTick
  (params (DeltaSeconds :type Float%20%28single-precision%29))
  (bind _hoveringamount (Variables|Hovering|GetHoveringAmount))
  ;[1 1 1] Event Tick
  ;[1 1 1] Hover
  (if (Variables|Hovering|GetShouldHover)
    (bind _floatalpha (Timeline|FloatingTimeline Play)
      (:Update
        (Transformation|AddWorldOffset (Variables|Default|GetStaticMesh) (Math|Vector|MakeVector (* _floatalpha (.x _hoveringamount)) (* _floatalpha (.y _hoveringamount)) (* _floatalpha (.z _hoveringamount))) true false)))))

(event EventPickup
  (params (AttachTo :type Scene%20Component%20Object%20Reference))
  ;[1 1 1] Event Pickup
  (if (not (Variables|Default|GetInHand))
    ;[1 1 1] Attach Object
    (Physics|SetSimulatePhysics (Variables|Default|GetStaticMesh) false)
    (bind _returnvalue (Transformation|AttachComponentToComponent (VehicleSound|GetRootComponent) AttachTo "None" "KeepWorld" "KeepWorld" "KeepWorld" false))
    (if _returnvalue
      (Variables|Default|SetInHand true)
      (Utilities|FlowControl|Sequence
        (:then_0
          ;[1 1 1] Disable gravity at pickup
          (Physics|SetEnableGravity (Variables|Default|GetStaticMesh) false)
          ;[1 1 1] Restore original hover status
          (Variables|Hovering|SetShouldHover (Variables|Hovering|GetShouldHoverStorage)))
        (:then_1
          ;[1 1 1] Make a copy, if picked up from the spawn
          (if (Variables|Default|GetShouldRespawn)
            (Game|SpawnActorfromClass (Utilities|GetClass self) (Variables|Default|GetSpawnTransform) "AlwaysSpawn" 0 0)
            (Variables|Default|SetShouldRespawn false)))))))

(event EventDrop
  (params (Momentum :type Transform) (MinSquaredLinearVelocity :type Float%20%28single-precision%29) (MinSquaredAngularVelocity :type Float%20%28single-precision%29))
  (bind _rotation (Math|Transform|BreakTransform Momentum))
  ;[1 1 1] Event Drop
  ;[1 1 1] Detach Object
  (Transformation|DetachFromActor "KeepWorld" "KeepWorld" "KeepWorld")
  (Variables|Default|SetInHand false)
  (Physics|SetSimulatePhysics (Variables|Default|GetStaticMesh) true)
  ;[1 1 1] Reset linear velocity if needed
  (if (< (Math|Vector|VectorLengthSquared (.Location (Math|Transform|BreakTransform Momentum))) MinSquaredLinearVelocity)
    (Physics|SetPhysicsLinearVelocity (Variables|Default|GetStaticMesh) "0, 0, 0" false "None"))
  ;[1 1 1] Reset angular velocity if needed
  (if (< (+ (Math|Float|Square (.roll _rotation)) (Math|Float|Square (.pitch _rotation)) (Math|Float|Square (.yaw _rotation))) MinSquaredAngularVelocity)
    (Class|PrimitiveComponent|SetPhysicsAngularVelocityinDegrees (Variables|Default|GetStaticMesh) "0, 0, 0" false "None")))

(fn ConstructionScript)

(fn SwitchGravity
  (bind _staticmesh (Variables|Default|GetStaticMesh))
  (Physics|SetEnableGravity _staticmesh (not (Class|PrimitiveComponent|IsGravityEnabled _staticmesh))))