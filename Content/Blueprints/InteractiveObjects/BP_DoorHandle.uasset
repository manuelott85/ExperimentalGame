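; Grabbable door handle that swings its referenced door as the player moves it.
; While held, Tick sets the door mesh's world yaw from the pivot-to-handle angle via atan2, adding 180 degrees for mirrored scale.
; Rotation only updates while the door's current angle is within its open/closed limits plus a small tolerance.
; Pickup and Drop play the door's open/close sounds; when released, the handle teleports to the door's sphere each tick.
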(event EventBeginPlay
  (|CallParentFunction) ; This node is disabled and will not be called.\nDrag off pins to build functionality.
)

(event Collision|EventActorBeginOverlap
  (params (OtherActor :type Actor%20Object%20Reference)))

(event EventTick
  (params (DeltaSeconds :type Float%20%28single-precision%29))
  (bind _returnvalue (Transformation|GetActorLocation))
  (bind _meshtorotate (Variables|Default|GetMeshToRotate))
  (bind _returnvalue_2 (Transformation|GetActorScale3D _meshtorotate))
  (bind _staticmesh (Variables|/Game/Blueprints/InteractiveObjects/BP_DoorBase.BP_DoorBase_C|GetStaticMesh _meshtorotate))
  (bind _currentrelativerotation (Variables|/Game/Blueprints/InteractiveObjects/BP_DoorBase.BP_DoorBase_C|GetCurrentRelativeRotation _meshtorotate))
  (bind _returnvalue_3 (Transformation|GetWorldLocation _staticmesh))
  (bind _returnvalue_4 (- _returnvalue _returnvalue_3))
  (|CallParentFunction DeltaSeconds)
  (if (Variables|Default|GetShouldUpdateRotation)
    ;[1 1 1] Update Rotation
    (Variables|Default|SetNewYaw (Class|KismetMathLibrary|DegAtan2 (.y _returnvalue_4) (.x _returnvalue_4)))
    (if (and (< _currentrelativerotation (+ (Variables|/Game/Blueprints/InteractiveObjects/BP_DoorBase.BP_DoorBase_C|GetDoorOpenRotation _meshtorotate) 5.0)) (> _currentrelativerotation (- (Variables|/Game/Blueprints/InteractiveObjects/BP_DoorBase.BP_DoorBase_C|GetDoorClosedRotation _meshtorotate) 5.0)))
      (if (Math|Boolean|ORBoolean (< (.x _returnvalue_2) 0.0) (< (.y _returnvalue_2) 0.0) (< (.z _returnvalue_2) 0.0))
        (Transformation|SetWorldRotation _staticmesh (Math|Rotator|MakeRotator 0.0 0.0 (+ (Variables|Default|GetNewYaw) 1.8e+02)) false false)
        (else
          (Transformation|SetWorldRotation _staticmesh (Math|Rotator|MakeRotator 0.0 0.0 (Variables|Default|GetNewYaw)) false false))))
    (else
      ;[1 1 1] Move Handle back to the door
      (Transformation|SetActorLocation (Transformation|GetWorldLocation (Variables|/Game/Blueprints/InteractiveObjects/BP_DoorBase.BP_DoorBase_C|GetSphere (Variables|Default|GetMeshToRotate))) false true))))

(event EventPickup
  (params (AttachTo :type Scene%20Component%20Object%20Reference))
  (|CallParentFunction AttachTo)
  (Variables|Default|SetShouldUpdateRotation true)
  (Audio|Components|Audio|Play (Variables|/Game/Blueprints/InteractiveObjects/BP_DoorBase.BP_DoorBase_C|GetDoorOpen (Variables|Default|GetMeshToRotate)) 0.0))

(event EventDrop
  (params (Momentum :type Transform) (MinSquaredLinearVelocity :type Float%20%28single-precision%29) (MinSquaredAngularVelocity :type Float%20%28single-precision%29))
  (|CallParentFunction Momentum MinSquaredLinearVelocity MinSquaredAngularVelocity)
  (Variables|Default|SetShouldUpdateRotation false)
  (Audio|Components|Audio|Play (Variables|/Game/Blueprints/InteractiveObjects/BP_DoorBase.BP_DoorBase_C|GetDoorClose (Variables|Default|GetMeshToRotate)) 0.0))

(fn ConstructionScript
  (|CallParentFunction))