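; Interactive button component that physically sinks when pushed by an overlapping component, firing a Pressed event and a sound at full depth.
; Overlap handlers track the first overlapping component and its initial location, clearing it when that component leaves.
; Tick converts its movement into clamped local-Z press depth on ButtonRoot, or eases the button back when nothing overlaps.
; A DoOnce limits activation until press depth drops below maximum.
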(event OnComponentBeginOverlap(Button)
  (params (OverlappedComponent :type Primitive%20Component%20Object%20Reference) (OtherActor :type Actor%20Object%20Reference) (OtherComp :type Primitive%20Component%20Object%20Reference) (OtherBodyIndex :type Integer) (bFromSweep :type Boolean) (SweepResult :type Hit%20Result%20Structure%20%28by%20ref%29)))

(event OnComponentEndOverlap(Button)
  (params (OverlappedComponent :type Primitive%20Component%20Object%20Reference) (OtherActor :type Actor%20Object%20Reference) (OtherComp :type Primitive%20Component%20Object%20Reference) (OtherBodyIndex :type Integer)))

(event Custom|Button_EndOverlap
  (params (OtherComp :type Primitive%20Component%20Object%20Reference))
  (if (== OtherComp (Variables|Default|GetOverlappedComponent))
    (Variables|Default|SetOverlappedComponent 0)))

(event Custom|Button_BeginOverlap
  (params (OtherComp :type Primitive%20Component%20Object%20Reference))
  (Utilities|IsValid (Variables|Default|GetOverlappedComponent)
    (:Is%20Not%20Valid
      (bind _output_get (Variables|Default|SetOverlappedComponent OtherComp))
      (Variables|Default|SetInitialOverlapLocation (Transformation|GetWorldLocation _output_get)))))

(event EventTick
  (params (DeltaSeconds :type Float%20%28single-precision%29))
  (bind _buttonroot (Variables|Default|GetButtonRoot))
  (bind _returnvalue (Transformation|GetWorldTransform _buttonroot))
  (Utilities|FlowControl|Sequence
    (:then_0
      (Utilities|IsValid (Variables|Default|GetOverlappedComponent)
        (:Is%20Valid
          ;[1 1 1] Pressing the button
          (bind _output_get (Variables|Default|SetButtonPressedAmount (Math|Float|Clamp(Float) (.z (- (Math|Transform|InverseTransformLocation _returnvalue (Variables|Default|GetInitialOverlapLocation)) (Math|Transform|InverseTransformLocation _returnvalue (Transformation|GetWorldLocation (Variables|Default|GetOverlappedComponent))))) 0.0 (Variables|Default|GetMaxButtonPressAmount))))
          (Transformation|SetRelativeLocation (Variables|Default|GetButton) (Math|Vector|MakeVector 0.0 0.0 (* _output_get -1.0)) false false))
        (:Is%20Not%20Valid
          ;[1 1 1] Releasing the button
          (Transformation|SetRelativeLocation (Variables|Default|GetButton) (Math|Interpolation|VInterpTo (Variables|/Script/Engine.SceneComponent|GetRelativeLocation (Variables|Default|GetButton)) "0, 0, 0" DeltaSeconds 1e+01) false false))))
    (:then_1
      ;[1 1 1] Activating the button
      (if (>= (Variables|Default|GetButtonPressedAmount) (Variables|Default|GetMaxButtonPressAmount))
        (Utilities|FlowControl|DoOnce false :!label _label
          (:Completed
            (Default|CallPressed)
            (Audio|Components|Audio|Play (Variables|Default|GetButtonSound) 0.0)))
        (else
          (goto _label Reset))))))