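; BP_Handle is a grabbable handle that lets the player swing a BP_DoorBase door by pulling on it.
; Pickup and Drop toggle a flag that Tick reads to choose between driving the door and following it.
; While held, Tick sets the door mesh's yaw from the atan2 angle toward the handle, clamped between the door's closed and open rotations.
; Otherwise, Tick teleports the handle back to the door's Sphere component every frame.
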(event EventBeginPlay
  (|CallParentFunction) ; This node is disabled and will not be called.\nDrag off pins to build functionality.
)

(event Collision|EventActorBeginOverlap
  (params (OtherActor :type Actor%20Object%20Reference)))

(event EventTick
  (params (DeltaSeconds :type Float%20%28single-precision%29))
  (|CallParentFunction DeltaSeconds)
  (if (Variables|Default|GetShouldUpdateRotation)
    ;[1 1 1] Update Rotation
    (bind _asbp_door_base (Utilities|Casting|CastToBP_DoorBase (Variables|Default|GetMeshToRotate)))
    (Transformation|SetWorldRotation (Variables|/Game/Blueprints/BP_DoorBase.BP_DoorBase_C|GetStaticMesh _asbp_door_base) (Math|Rotator|MakeRotator 0.0 0.0 (Math|Float|Clamp(Float) (Class|KismetMathLibrary|DegAtan2 (.y (- (Transformation|GetActorLocation) (Transformation|GetWorldLocation (Variables|/Game/Blueprints/BP_DoorBase.BP_DoorBase_C|GetStaticMesh _asbp_door_base)))) (.x (- (Transformation|GetActorLocation) (Transformation|GetWorldLocation (Variables|/Game/Blueprints/BP_DoorBase.BP_DoorBase_C|GetStaticMesh _asbp_door_base))))) (Variables|/Game/Blueprints/BP_DoorBase.BP_DoorBase_C|GetDoorClosedRotation _asbp_door_base) (Variables|/Game/Blueprints/BP_DoorBase.BP_DoorBase_C|GetDoorOpenRotation _asbp_door_base))) false false)
    (else
      ;[1 1 1] Move Handle back to the door
      (bind _asbp_door_base_2 (Utilities|Casting|CastToBP_DoorBase (Variables|Default|GetMeshToRotate)))
      (Transformation|SetActorLocation (Transformation|GetWorldLocation (Variables|/Game/Blueprints/BP_DoorBase.BP_DoorBase_C|GetSphere _asbp_door_base_2)) false true))))

(event EventPickup
  (params (AttachTo :type Scene%20Component%20Object%20Reference))
  (|CallParentFunction AttachTo)
  (Variables|Default|SetShouldUpdateRotation true))

(event EventDrop
  (params (Momentum :type Transform) (MinSquaredLinearVelocity :type Float%20%28single-precision%29) (MinSquaredAngularVelocity :type Float%20%28single-precision%29))
  (|CallParentFunction Momentum MinSquaredLinearVelocity MinSquaredAngularVelocity)
  (Variables|Default|SetShouldUpdateRotation false))

(fn ConstructionScript
  (|CallParentFunction))