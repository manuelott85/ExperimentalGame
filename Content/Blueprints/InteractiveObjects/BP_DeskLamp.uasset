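; BP_DeskLamp is an interactive desk lamp that switches on and off with a button.
; On BeginPlay it creates a dynamic material for the bulb with emission at zero and configures CompInteractiveButton with its audio and button parts.
; Button overlaps are forwarded to that component, whose Pressed event calls SwitchLight.
; SwitchLight toggles the spotlight and derives the bulb's emission intensity from the light's visibility.
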(event OnComponentBeginOverlap(Button)
  (params (OverlappedComponent :type Primitive%20Component%20Object%20Reference) (OtherActor :type Actor%20Object%20Reference) (OtherComp :type Primitive%20Component%20Object%20Reference) (OtherBodyIndex :type Integer) (bFromSweep :type Boolean) (SweepResult :type Hit%20Result%20Structure%20%28by%20ref%29))
  (Default|ButtonBeginOverlap (Variables|Default|GetComp_InteractiveButton) OtherComp))

(event OnComponentEndOverlap(Button)
  (params (OverlappedComponent :type Primitive%20Component%20Object%20Reference) (OtherActor :type Actor%20Object%20Reference) (OtherComp :type Primitive%20Component%20Object%20Reference) (OtherBodyIndex :type Integer))
  (Default|ButtonEndOverlap (Variables|Default|GetComp_InteractiveButton) OtherComp))

(event Custom|SwitchLight
  (bind _spotlight (Variables|Default|GetSpotLight))
  (Rendering|ToggleVisibility _spotlight false)
  (Rendering|Material|SetScalarParameterValue (Variables|Default|GetAssignedDynamicMaterial) "Emission Intensity" (* (Math|Conversions|ToFloat(Boolean) (Variables|/Script/Engine.SceneComponent|GetbVisible _spotlight)) 1e+01) :!class /Script/Engine.MaterialInstanceDynamic))

(event EventBeginPlay
  (bind _bulp (Variables|Default|GetBulp))
  (bind _comp_interactivebutton (Variables|Default|GetComp_InteractiveButton))
  ;[1 1 1] Begin Play
  (|CallParentFunction)
  (Utilities|FlowControl|Sequence
    (:then_0
      (bind _returnvalue (Rendering|Material|CreateDynamicMaterialInstance _bulp (Rendering|Material|GetMaterial _bulp 0) "None" :!class /Script/Engine.KismetMaterialLibrary))
      (bind _output_get (Variables|Default|SetAssignedDynamicMaterial _returnvalue))
      (Rendering|Material|SetMaterial (Variables|Default|GetBulp) 0 _output_get)
      (Rendering|Material|SetScalarParameterValue (Variables|Default|GetAssignedDynamicMaterial) "Emission Intensity" 0.0 :!class /Script/Engine.MaterialInstanceDynamic))
    (:then_1
      (Variables|/Game/Blueprints/InteractiveObjects/Comp_InteractiveButton.Comp_InteractiveButton_C|SetButtonSound _comp_interactivebutton (Variables|Default|GetAudio))
      (Variables|/Game/Blueprints/InteractiveObjects/Comp_InteractiveButton.Comp_InteractiveButton_C|SetButtonRoot _comp_interactivebutton (Variables|Default|GetButtonRoot))
      (Variables|/Game/Blueprints/InteractiveObjects/Comp_InteractiveButton.Comp_InteractiveButton_C|SetButton _comp_interactivebutton (Variables|Default|GetButton))
      (EventDispatchers|BindEventtoPressed _comp_interactivebutton (delegate Custom|SwitchLight)))))

(fn ConstructionScript)