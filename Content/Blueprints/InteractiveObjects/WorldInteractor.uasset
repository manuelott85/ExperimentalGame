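; WorldInteractor is a component on a VR motion controller that lets it hover and drag world objects.
; While enabled, each tick it sphere-overlaps dynamic and physics objects, ignoring both controllers, and takes the first hit as the hovered object.
; Hover changes end any drag and send unhover and hover messages; StartDrag and StopDrag gate a per-tick drag message to that object.
; The hovered object persists when nothing overlaps.
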(event Custom|Enable
  (Utilities|FlowControl|Gate false) ; enters at Open
)

(event Custom|Disable
  (Utilities|FlowControl|Gate false) ; enters at Close
)

(event Custom|StartDrag
  (Variables|Default|SetDragging true)
  (Class|WorldInteractionInterface|OnDragStart(Message) (Variables|Default|GetHoveredObject) self)
  (Utilities|FlowControl|Gate true) ; enters at Open
)

(event Custom|StopDrag
  (if (Variables|Default|GetDragging)
    (Variables|Default|SetDragging false)
    (Class|WorldInteractionInterface|OnDragEnd(Message) (Variables|Default|GetHoveredObject) self)
    (Utilities|FlowControl|Gate true) ; enters at Close
  ))

(event EventTick
  (params (DeltaSeconds :type Float%20%28single-precision%29))
  (Utilities|FlowControl|Gate false
    (:Exit
      (Utilities|FlowControl|Sequence
        (:then_0
          ;[1 1 1] Sphere overlap
          (bind _asmotion_controller_pawn (Utilities|Casting|CastToMotionControllerPawn (Components|GetOwner (Components|GetOwner))))
          (bind (_outactors _returnvalue) (Collision|SphereOverlapActors (Transformation|GetWorldLocation) (Variables|Default|GetRadius) (Utilities|Array|MakeArray "ObjectTypeQuery2" "ObjectTypeQuery4") 0 (Utilities|Array|MakeArray (Variables|/Game/Blueprints/MotionControllerPawn.MotionControllerPawn_C|GetLeftController _asmotion_controller_pawn) (Variables|/Game/Blueprints/MotionControllerPawn.MotionControllerPawn_C|GetRightController _asmotion_controller_pawn))))
          (if _returnvalue
            ;[1 1 1] Hover Messages
            (if (!= (Variables|Default|GetHoveredObject) (Utilities|Array|Get(acopy) _outactors))
              (Class|WorldInteractionInterface|OnUnhover(Message) (Variables|Default|GetHoveredObject) self)
              (CallFunction|StopDrag)
              (bind _output_get (Variables|Default|SetHoveredObject (Utilities|Array|Get(acopy) _outactors)))
              (Class|WorldInteractionInterface|OnHover(Message) _output_get self))))
        (:then_1
          (Utilities|FlowControl|Gate true
            (:Exit
              (Class|WorldInteractionInterface|OnDrag(Message) (Variables|Default|GetHoveredObject) self))))))))