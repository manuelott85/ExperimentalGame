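; Grabbable handle actor that lets the player drag a linked drawer or door, held in MeshToMove.
; Pickup and Drop extend the parent events, starting or stopping the drag with the handle's Sphere and toggling ShouldUpdateLocation.
; While held, Tick tells MeshToMove to update its location.
; Otherwise, Tick teleports the handle back to the mesh's HandlePos every frame, keeping it attached without parenting.
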(event EventBeginPlay
  (|CallParentFunction) ; This node is disabled and will not be called.\nDrag off pins to build functionality.
)

(event Collision|EventActorBeginOverlap
  (params (OtherActor :type Actor%20Object%20Reference)))

(event EventTick
  (params (DeltaSeconds :type Float%20%28single-precision%29))
  (|CallParentFunction DeltaSeconds)
  (if (Variables|Default|GetShouldUpdateLocation)
    (Default|UpdateLocation (Variables|Default|GetMeshToMove))
    (else
      ;[1 1 1] Move Handle back to the door
      (Transformation|SetActorLocation (Transformation|GetWorldLocation (Variables|/Game/Blueprints/InteractiveObjects/BP_DrawerBase.BP_DrawerBase_C|GetHandlePos (Variables|Default|GetMeshToMove))) false true))))

(event EventPickup
  (params (AttachTo :type Scene%20Component%20Object%20Reference))
  (|CallParentFunction AttachTo)
  (Default|StartDragging (Variables|Default|GetMeshToMove) (Variables|Default|GetSphere))
  (Variables|Default|SetShouldUpdateLocation true))

(event EventDrop
  (params (Momentum :type Transform) (MinSquaredLinearVelocity :type Float%20%28single-precision%29) (MinSquaredAngularVelocity :type Float%20%28single-precision%29))
  (|CallParentFunction Momentum MinSquaredLinearVelocity MinSquaredAngularVelocity)
  (Default|StopDragging (Variables|Default|GetMeshToMove) (Variables|Default|GetSphere))
  (Variables|Default|SetShouldUpdateLocation false))

(fn ConstructionScript
  (|CallParentFunction))