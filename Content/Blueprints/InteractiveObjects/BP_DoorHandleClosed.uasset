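; A pickup handle for a closed, locked door that cannot be carried away.
; On BeginPlay it records its spawn location.
; Pickup runs the parent grab logic and plays the Locked audio or effect component if it is not already playing.
; Drop runs the parent release, then teleports the handle back to its spawn location on the door.
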(event EventBeginPlay
  (|CallParentFunction)
  (Variables|Default|SetSpawnPosition (Transformation|GetActorLocation)))

(event EventTick
  (params (DeltaSeconds :type Float%20%28single-precision%29))
  (|CallParentFunction DeltaSeconds))

(event EventPickup
  (params (AttachTo :type Scene%20Component%20Object%20Reference))
  (bind _locked (Variables|Default|GetLocked))
  (|CallParentFunction AttachTo)
  (if (not (Audio|Components|Audio|IsPlaying _locked))
    (Audio|Components|Audio|Play _locked 0.0)))

(event EventDrop
  (params (Momentum :type Transform) (MinSquaredLinearVelocity :type Float%20%28single-precision%29) (MinSquaredAngularVelocity :type Float%20%28single-precision%29))
  (|CallParentFunction Momentum MinSquaredLinearVelocity MinSquaredAngularVelocity)
  ;[1 1 1] Move Handle back to the door
  (Transformation|SetActorLocation (Variables|Default|GetSpawnPosition) false true))

(fn ConstructionScript
  (|CallParentFunction))