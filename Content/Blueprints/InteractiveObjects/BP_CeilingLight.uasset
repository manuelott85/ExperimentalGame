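; BP_CeilingLight is an interactive ceiling lamp that a referenced light switch turns on and off.
; On BeginPlay it creates a dynamic material for the colored glass mesh, sets its emission to the configured intensity and, if the switch reference is valid, binds to its on/off events.
; Those events toggle the point light's visibility and switch the glass emission between that intensity and zero.
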(event Custom|SwitchOn
  (Rendering|SetVisibility (Variables|Default|GetPointLight) true false)
  (Rendering|Material|SetScalarParameterValue (Variables|Default|GetAssignedDynamicMaterial) "Emission Intensity" (Variables|Default|GetEmission%20Intensity) :!class /Script/Engine.MaterialInstanceDynamic))

(event Custom|SwitchOff
  (Rendering|SetVisibility (Variables|Default|GetPointLight) false false)
  (Rendering|Material|SetScalarParameterValue (Variables|Default|GetAssignedDynamicMaterial) "Emission Intensity" 0.0 :!class /Script/Engine.MaterialInstanceDynamic))

(event EventBeginPlay
  (bind _lightswitchreference (Variables|Default|GetLightSwitchReference))
  (bind _sm_lampceiling_colored_glass (Variables|Default|GetSM_LampCeiling_Colored_Glass))
  ;[1 1 1] Create Dynamic Material to be able to use its paramters
  (bind _returnvalue (Rendering|Material|CreateDynamicMaterialInstance _sm_lampceiling_colored_glass (Rendering|Material|GetMaterial _sm_lampceiling_colored_glass 0) "None" :!class /Script/Engine.KismetMaterialLibrary))
  (bind _output_get (Variables|Default|SetAssignedDynamicMaterial _returnvalue))
  (Rendering|Material|SetMaterial (Variables|Default|GetSM_LampCeiling_Colored_Glass) 0 _output_get)
  (Rendering|Material|SetScalarParameterValue (Variables|Default|GetAssignedDynamicMaterial) "Emission Intensity" (Variables|Default|GetEmission%20Intensity) :!class /Script/Engine.MaterialInstanceDynamic)
  ;[1 1 1] Bind the switch
  (Utilities|IsValid _lightswitchreference
    (:Is%20Valid
      (EventDispatchers|BindEventtoSwitchedon _lightswitchreference (delegate Custom|SwitchOn))
      (EventDispatchers|BindEventtoSwitchedOff _lightswitchreference (delegate Custom|SwitchOff)))))

(fn ConstructionScript)