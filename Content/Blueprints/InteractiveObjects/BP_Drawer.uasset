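; Interactive drawer that slides along its Box's right vector as the component overlapping that Box moves.
; BeginPlay sets the closed-to-open segment from DrawingDistance, and overlap begin/end captures or releases one interactor, saving the drawer's position on release.
; Tick applies the interactor's signed, axis-weighted offset only when the target lies on that segment, otherwise printing the deviation.
; An alternative physics-based clamp is left unconnected.
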(event OnComponentBeginOverlap(Box)
  (params (OverlappedComponent :type Primitive%20Component%20Object%20Reference) (OtherActor :type Actor%20Object%20Reference) (OtherComp :type Primitive%20Component%20Object%20Reference) (OtherBodyIndex :type Integer) (bFromSweep :type Boolean) (SweepResult :type Hit%20Result%20Structure%20%28by%20ref%29))
  (Utilities|IsValid (Variables|Default|GetCurrentInteractor)
    (:Is%20Not%20Valid
      (Variables|Default|SetInitialInteractorLocation (Transformation|GetWorldLocation OtherComp))
      (Variables|Default|SetCurrentInteractor OtherComp))))

(event OnComponentEndOverlap(Box)
  (params (OverlappedComponent :type Primitive%20Component%20Object%20Reference) (OtherActor :type Actor%20Object%20Reference) (OtherComp :type Primitive%20Component%20Object%20Reference) (OtherBodyIndex :type Integer))
  (if (== OtherComp (Variables|Default|GetCurrentInteractor))
    (Variables|Default|SetCurrentInteractor 0)
    (Variables|Default|SetLastDrawerLocation (Transformation|GetWorldLocation (Variables|Default|GetBox)))))

(event EventBeginPlay
  (bind _box (Variables|Default|GetBox))
  ;[1 1 1] Begin Play
  (bind _output_get (Variables|Default|SetLastDrawerLocation (Transformation|GetWorldLocation _box)))
  (bind _output_get_2 (Variables|Default|SetInitialDrawerLocation _output_get))
  (Variables|Default|SetMaxDrawerLocation (+ _output_get_2 (* (Math|Vector|GetRightVector _box) (Variables|Default|GetDrawingDistance)))))

(event EventTick
  (params (DeltaSeconds :type Float%20%28single-precision%29))
  (bind _initialinteractorlocation (Variables|Default|GetInitialInteractorLocation))
  (bind _currentinteractor (Variables|Default|GetCurrentInteractor))
  (bind _box (Variables|Default|GetBox))
  (bind _box_2 (Variables|Default|GetBox))
  (bind _returnvalue (Math|Vector|GetRightVector _box))
  (bind _returnvalue_2 (Transformation|GetWorldLocation _currentinteractor))
  (bind _returnvalue_3 (- _initialinteractorlocation _returnvalue_2))
  (bind _returnvalue_4 (* _returnvalue_3 _returnvalue))
  (bind _returnvalue_5 (Math|Vector|VectorLength _returnvalue_4))
  ;[1 1 1] Event Tick
  (Utilities|IsValid _currentinteractor
    (:Is%20Valid
      (if (< (Math|Vector|DotProduct (Math|Vector|Normalize _returnvalue_3) _returnvalue) 0.0)
        (Variables|Default|SetDistance (* _returnvalue_5 -1.0))
        (else
          (Variables|Default|SetDistance _returnvalue_5)))
      (if (< (Class|KismetMathLibrary|GetPointDistancetoSegment (- (Variables|Default|GetLastDrawerLocation) (* (Math|Vector|GetRightVector _box_2) (Variables|Default|GetDistance))) (Variables|Default|GetInitialDrawerLocation) (Variables|Default|GetMaxDrawerLocation)) 1.0)
        (Transformation|SetWorldLocation _box_2 (- (Variables|Default|GetLastDrawerLocation) (* (Math|Vector|GetRightVector _box_2) (Variables|Default|GetDistance))) false false)
        (else
          (Development|PrintString (Utilities|String|ToString(Float) (Class|KismetMathLibrary|GetPointDistancetoSegment (- (Variables|Default|GetLastDrawerLocation) (* (Math|Vector|GetRightVector _box_2) (Variables|Default|GetDistance))) (Variables|Default|GetInitialDrawerLocation) (Variables|Default|GetMaxDrawerLocation)))))))))

(fn ConstructionScript)