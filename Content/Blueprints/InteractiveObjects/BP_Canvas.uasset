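; BP_Canvas is an interactive canvas that displays a random silhouette from an array on its Drawer component.
; On BeginPlay it creates a dynamic material for the Drawer, picks an initial silhouette and binds re-picking to the MaxReached event.
; Each pick waits on a short retriggerable delay, rerolls until the index differs from the last one, then sets the material's Silhouette texture parameter.
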(event Custom|Assign%20random%20Silhouette
  (Utilities|FlowControl|RetriggerableDelay 0.1)
  (while (== (Variables|Default|GetLastIndex) (Variables|Default|GetcurrentIndex))
    (Variables|Default|SetcurrentIndex (Math|Random|RandomIntegerinRange 0 (- (Utilities|Array|Length (Variables|Default|GetSilhouetteArray)) 1))))
  (Rendering|Material|SetTextureParameterValue (Variables|Default|GetAssignedDynamicMaterial) "Silhouette" (Utilities|Array|Get(acopy) (Variables|Default|GetSilhouetteArray) (Variables|Default|GetcurrentIndex)))
  (Variables|Default|SetLastIndex (Variables|Default|GetcurrentIndex)))

(event EventBeginPlay
  (bind _drawer (Variables|Default|GetDrawer))
  (|CallParentFunction)
  (Utilities|FlowControl|Sequence
    (:then_0
      ;[1 1 1] Create and store the dynamic material
      (bind _returnvalue (Rendering|Material|CreateDynamicMaterialInstance _drawer (Rendering|Material|GetMaterial _drawer 0) "None" :!class /Script/Engine.KismetMaterialLibrary))
      (bind _output_get (Variables|Default|SetAssignedDynamicMaterial _returnvalue))
      (Rendering|Material|SetMaterial (Variables|Default|GetDrawer) 0 _output_get))
    (:then_1
      (CallFunction|AssignRandomSilhouette))
    (:then_2
      (EventDispatchers|BindEventtoMaxReached (delegate Custom|Assign%20random%20Silhouette)))))

(fn ConstructionScript
  (|CallParentFunction))