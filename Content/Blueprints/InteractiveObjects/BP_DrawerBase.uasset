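; Base Blueprint for a drawer that an interactor drags open and closed along the box's right vector.
; StartDragging and StopDragging track the interactor, save the drawer position and play open/close audio.
; UpdateLocation projects interactor movement onto that axis, moving the box only within the DrawingDistance segment and otherwise calling MaxReached or MinReached.
; An unconnected physics-based clamp on relative X remains unused.
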(event Custom|UpdateLocation
  (bind _initialinteractorlocation (Variables|Default|GetInitialInteractorLocation))
  (bind _currentinteractor (Variables|Default|GetCurrentInteractor))
  (bind _box (Variables|Default|GetBox))
  (bind _box_2 (Variables|Default|GetBox))
  (bind _returnvalue (Math|Vector|GetRightVector _box))
  (bind _returnvalue_2 (Transformation|GetWorldLocation _currentinteractor))
  (bind _returnvalue_3 (- _initialinteractorlocation _returnvalue_2))
  (bind _returnvalue_4 (* _returnvalue_3 _returnvalue))
  (bind _returnvalue_5 (Math|Vector|VectorLength _returnvalue_4))
  (Utilities|IsValid _currentinteractor
    (:Is%20Valid
      (if (< (Math|Vector|DotProduct (Math|Vector|Normalize _returnvalue_3 0.01) _returnvalue) 0.0)
        (Variables|Default|SetDistance (* _returnvalue_5 -1.0))
        (else
          (Variables|Default|SetDistance _returnvalue_5)))
      (Variables|Default|SetNewLocation (- (Variables|Default|GetLastDrawerLocation) (* (Math|Vector|GetRightVector _box_2) (Variables|Default|GetDistance))))
      (if (< (Class|KismetMathLibrary|GetPointDistancetoSegment (Variables|Default|GetNewLocation) (Variables|Default|GetInitialDrawerLocation) (Variables|Default|GetMaxDrawerLocation)) 1.0)
        (Transformation|SetWorldLocation _box_2 (Variables|Default|GetNewLocation) false false)
        (elif (< (Math|Vector|Distance(Vector) (Variables|Default|GetNewLocation) (Variables|Default|GetMaxDrawerLocation)) (Math|Vector|Distance(Vector) (Variables|Default|GetNewLocation) (Variables|Default|GetInitialDrawerLocation)))
          (Default|CallMaxReached)
          (else
            (Default|CallMinReached)))))))

(event Custom|StopDragging
  (params (Interactor :type Scene%20Component%20Object%20Reference))
  (if (== Interactor (Variables|Default|GetCurrentInteractor))
    (Variables|Default|SetCurrentInteractor 0)
    (Variables|Default|SetLastDrawerLocation (Transformation|GetWorldLocation (Variables|Default|GetBox)))
    (Audio|Components|Audio|Play (Variables|Default|GetDrawerClose) 0.0)))

(event Custom|StartDragging
  (params (Interactor :type Scene%20Component%20Object%20Reference))
  (Utilities|IsValid (Variables|Default|GetCurrentInteractor)
    (:Is%20Not%20Valid
      (Variables|Default|SetInitialInteractorLocation (Transformation|GetWorldLocation Interactor))
      (Variables|Default|SetCurrentInteractor Interactor)
      (Audio|Components|Audio|Play (Variables|Default|GetDrawerOpen) 0.0))))

(event EventBeginPlay
  (bind _box (Variables|Default|GetBox))
  ;[1 1 1] Begin Play
  (bind _output_get (Variables|Default|SetLastDrawerLocation (Transformation|GetWorldLocation _box)))
  (bind _output_get_2 (Variables|Default|SetInitialDrawerLocation _output_get))
  (Variables|Default|SetMaxDrawerLocation (+ _output_get_2 (* (Math|Vector|GetRightVector _box) (Variables|Default|GetDrawingDistance)))))

(fn ConstructionScript)