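; BP_DoorBase is a base Blueprint for a physics-driven swinging door that keeps its yaw within set limits.
; Each Tick, it converts the mesh's world rotation into the root's space and compares the yaw with DoorClosedRotation and DoorOpenRotation.
; Past either limit, it snaps the mesh to that yaw with zero pitch and roll, then zeroes its angular velocity.
; BeginPlay records the starting yaw, which this graph never reads.
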(event EventBeginPlay
  (Variables|Default|SetInitialRotation (.yaw (Variables|/Script/Engine.SceneComponent|GetRelativeRotation (Variables|Default|GetStaticMesh)))))

(event EventTick
  (params (DeltaSeconds :type Float%20%28single-precision%29))
  (Variables|Default|SetCurrentRelativeRotation (.yaw (Math|Transform|InverseTransformRotation (Transformation|GetWorldTransform (Variables|Default|GetDefaultSceneRoot)) (Transformation|GetWorldRotation (Variables|Default|GetStaticMesh)))))
  (if (< (Variables|Default|GetCurrentRelativeRotation) (Variables|Default|GetDoorClosedRotation))
    (Transformation|SetWorldRotation (Variables|Default|GetStaticMesh) (Math|Rotator|MakeRotator 0.0 0.0 (+ (.yaw (Transformation|GetWorldRotation (Variables|Default|GetDefaultSceneRoot))) (Variables|Default|GetDoorClosedRotation))) false false)
    (Class|PrimitiveComponent|SetPhysicsAngularVelocityinDegrees (Variables|Default|GetStaticMesh) "0, 0, 0" false "None" :!label _label)
    (elif (> (Variables|Default|GetCurrentRelativeRotation) (Variables|Default|GetDoorOpenRotation))
      (Transformation|SetWorldRotation (Variables|Default|GetStaticMesh) (Math|Rotator|MakeRotator 0.0 0.0 (+ (.yaw (Transformation|GetWorldRotation (Variables|Default|GetDefaultSceneRoot))) (Variables|Default|GetDoorOpenRotation))) false false)
      (goto _label))))

(fn ConstructionScript)