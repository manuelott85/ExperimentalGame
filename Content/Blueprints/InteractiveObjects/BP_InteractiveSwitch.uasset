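; Interactive lever switch that follows an overlapping component and broadcasts SwitchedOn and SwitchedOff events.
; The first component to overlap LeverHandler is tracked until it leaves.
; Each tick, lever pitch combines the component's actor-space angle with its pitch change since overlap, clamped to limits.
; Exactly matching the activation or deactivation pitch fires the event and plays OnOff, repeating every tick while held there.
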(event OnComponentBeginOverlap(LeverHandler)
  (params (OverlappedComponent :type Primitive%20Component%20Object%20Reference) (OtherActor :type Actor%20Object%20Reference) (OtherComp :type Primitive%20Component%20Object%20Reference) (OtherBodyIndex :type Integer) (bFromSweep :type Boolean) (SweepResult :type Hit%20Result%20Structure%20%28by%20ref%29))
  (Utilities|IsValid (Variables|Default|GetOverlappedComponent)
    (:Is%20Not%20Valid
      (bind _output_get (Variables|Default|SetOverlappedComponent OtherComp))
      (Variables|Default|SetInitialOverlapLocation (Transformation|GetWorldLocation _output_get))
      (Variables|Default|SetInitialOverlapRotation (Transformation|GetWorldRotation _output_get)))))

(event OnComponentEndOverlap(LeverHandler)
  (params (OverlappedComponent :type Primitive%20Component%20Object%20Reference) (OtherActor :type Actor%20Object%20Reference) (OtherComp :type Primitive%20Component%20Object%20Reference) (OtherBodyIndex :type Integer))
  (if (== OtherComp (Variables|Default|GetOverlappedComponent))
    (Variables|Default|SetOverlappedComponent 0)))

(event EventBeginPlay
  ;[1 1 1] Begin Play
  ;[1 1 1] Store initial values
  (Variables|Default|SetInitialLeverRotation (Variables|/Script/Engine.SceneComponent|GetRelativeRotation (Variables|Default|GetLeverRotate))))

(event EventTick
  (params (DeltaSeconds :type Float%20%28single-precision%29))
  (bind _returnvalue (Transformation|GetActorTransform))
  (bind _overlappedcomponent (Variables|Default|GetOverlappedComponent))
  (bind _returnvalue_2 (Transformation|GetWorldLocation _overlappedcomponent))
  (bind _returnvalue_3 (Math|Transform|InverseTransformLocation _returnvalue _returnvalue_2))
  (bind _returnvalue_4 (Math|Vector|UnrotateVector _returnvalue_3 "90.000000, 0, 0"))
  ;[1 1 1] Event Tick
  (Utilities|IsValid (Variables|Default|GetOverlappedComponent)
    (:Is%20Valid
      (bind _output_get (Variables|Default|SetCurrentPitch (Math|Float|Clamp(Float) (+ (Class|KismetMathLibrary|DegAtan2 (.z _returnvalue_4) (.x _returnvalue_4)) (- (.pitch (Transformation|GetWorldRotation _overlappedcomponent)) (.pitch (Variables|Default|GetInitialOverlapRotation)))) (Variables|Default|GetMinPitch) (Variables|Default|GetMaxPitch))))
      (Transformation|SetRelativeRotation (Variables|Default|GetLeverRotate) (Math|Rotator|MakeRotator 0.0 _output_get 0.0) false false)
      (if (== (Variables|Default|GetCurrentPitch) (Variables|Default|GetActivationPitch))
        (Default|CallSwitchedon)
        (Audio|Components|Audio|Play (Variables|Default|GetOnOff) 0.0 :!label _label)
        (elif (== (Variables|Default|GetCurrentPitch) (Variables|Default|GetDeactivationPitch))
          (Default|CallSwitchedOff)
          (goto _label))))))

(fn ConstructionScript)