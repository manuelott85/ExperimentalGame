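; BP_AudienceCamera is a spectator camera for VR that renders to a render target and saves screenshots when its in-world button is pressed.
; After a two-second delay for hands to spawn, it hides every MotionControllerPawn and both its controllers from the SceneCaptureComponent2D.
; Button overlaps feed CompInteractiveButton, whose Pressed event exports the capture's render target as a timestamped PNG in the game source screenshots folder.
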(event OnComponentBeginOverlap(Button)
  (params (OverlappedComponent :type Primitive%20Component%20Object%20Reference) (OtherActor :type Actor%20Object%20Reference) (OtherComp :type Primitive%20Component%20Object%20Reference) (OtherBodyIndex :type Integer) (bFromSweep :type Boolean) (SweepResult :type Hit%20Result%20Structure%20%28by%20ref%29))
  (Default|ButtonBeginOverlap (Variables|Default|GetComp_InteractiveButton) OtherComp))

(event OnComponentEndOverlap(Button)
  (params (OverlappedComponent :type Primitive%20Component%20Object%20Reference) (OtherActor :type Actor%20Object%20Reference) (OtherComp :type Primitive%20Component%20Object%20Reference) (OtherBodyIndex :type Integer))
  (Default|ButtonEndOverlap (Variables|Default|GetComp_InteractiveButton) OtherComp))

(event Custom|TakeScreenhot
  (bind _returnvalue (Math|DateTime|Now))
  (Variables|Default|SetFilePath (Utilities|String|Append (Class|BlueprintPathsLibrary|GameSourceDir) "screenshots\\"))
  (Variables|Default|SetScreenshotName (Utilities|String|Append (Utilities|String|ToString(Integer) (.year _returnvalue)) "-" (Utilities|String|ToString(Integer) (.month _returnvalue)) "-" (Utilities|String|ToString(Integer) (.day _returnvalue)) "-" (Utilities|String|ToString(Integer) (.hour _returnvalue)) (Utilities|String|ToString(Integer) (.minute _returnvalue)) "-" (Utilities|String|ToString(Integer) (.second _returnvalue)) "-" (Utilities|String|ToString(Integer) (.millisecond _returnvalue)) ".png"))
  (Rendering|ExportRenderTarget (Variables|/Script/Engine.SceneCaptureComponent2D|GetTextureTarget (Variables|Default|GetSceneCaptureComponent2D)) (Variables|Default|GetFilePath) (Variables|Default|GetScreenshotName))
  (Development|PrintString (Utilities|String|Append "Screenshot saved: " (Variables|Default|GetFilePath) (Variables|Default|GetScreenshotName)) true true "(R=0.026147,G=1.000000,B=0.000000,A=1.000000)" 2e+01))

(event EventBeginPlay
  (bind _comp_interactivebutton (Variables|Default|GetComp_InteractiveButton))
  (bind _scenecapturecomponent2d (Variables|Default|GetSceneCaptureComponent2D))
  (bind _hiddenactors (Variables|/Script/Engine.SceneCaptureComponent|GetHiddenActors _scenecapturecomponent2d))
  (|CallParentFunction)
  (Utilities|FlowControl|Sequence
    (:then_0
      ;[1 1 1] Remove any playerPawns
      (Utilities|FlowControl|Delay 2.0) ; wait for the hands to spawn
      (bind _outactors (Actor|GetAllActorsOfClass "/Game/Blueprints/MotionControllerPawn.MotionControllerPawn_C"))
      (for _array_element _outactors
        (Utilities|Array|Add _hiddenactors _array_element)
        (Utilities|Array|Add _hiddenactors (Variables|/Game/Blueprints/MotionControllerPawn.MotionControllerPawn_C|GetLeftController _array_element))
        (Utilities|Array|Add _hiddenactors (Variables|/Game/Blueprints/MotionControllerPawn.MotionControllerPawn_C|GetRightController _array_element))))
    (:then_1
      ;[1 1 1] Setup Interactive Button
      (Variables|/Game/Blueprints/InteractiveObjects/Comp_InteractiveButton.Comp_InteractiveButton_C|SetButtonSound _comp_interactivebutton (Variables|Default|GetButtonAudio))
      (Variables|/Game/Blueprints/InteractiveObjects/Comp_InteractiveButton.Comp_InteractiveButton_C|SetButtonRoot _comp_interactivebutton (Variables|Default|GetButtonRoot))
      (Variables|/Game/Blueprints/InteractiveObjects/Comp_InteractiveButton.Comp_InteractiveButton_C|SetButton _comp_interactivebutton (Variables|Default|GetButton))
      (EventDispatchers|BindEventtoPressed _comp_interactivebutton (delegate Custom|TakeScreenhot)))))

(fn ConstructionScript
  (|CallParentFunction))